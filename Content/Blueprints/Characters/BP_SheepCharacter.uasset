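; BP_SheepCharacter is a sheep character Blueprint that reports elimination and scoring events to the game instance.
; On possession it initializes its input mapping context and caches a BP_GameInstance reference.
; Elimination disables the character and notifies the game instance, and a helper function awards the SheepNotIdentify score action to the player's controller through that same instance.
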(event `self.ReceivePossessed`
  (params (NewController :type "Controller Object Reference"))
  (`self.InitializeMappingContext`)
  (`self.InitializeVariables`))

(event `self.Eliminate`
  (`self.DisableCharacter`)
  (`/Game/Blueprints/GameMode/BP_GameInstance.SheepElimination` (`self.GameInstance`)))

(fn `AddNotIdentifyScore`
  (`/Game/Blueprints/GameMode/BP_GameInstance.AddScoreActionToPlayer` (`self.GameInstance`) (`self.PlayerController`) "ESA_SheepNotIdentify"))

(fn `InitializeVariables`
  (bind _asbp_game_instance (cast `/Game/Blueprints/GameMode/BP_GameInstance` (`GameplayStatics.GetGameInstance`)))
  (set `self.GameInstance` _asbp_game_instance))

(fn `UserConstructionScript`)