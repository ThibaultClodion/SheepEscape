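; BP_SheepInWater is an actor that plays a sheep sinking and drowning after it drops into water.
; DropInWater waits a configurable delay, turns on the drowning flag, then waits a lifetime before destroying the actor.
; While drowning, Tick lowers the actor along local Z by DrownSpeed each frame, without delta-time scaling.
; Initialize sets the delay, sink speed and lifetime from outside.
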(event `DropInWater`
  (`KismetSystemLibrary.Delay` (`self.TimeBeforeDrown`))
  (set `self.IsDrowing` true)
  (`KismetSystemLibrary.Delay` (`self.LifetimeAfterDrown`))
  (`self.K2_DestroyActor`))

(event `self.ReceiveTick`
  (params (DeltaSeconds :type "Float (single-precision)"))
  (if (`self.IsDrowing`)
    (`self.K2_AddActorLocalOffset` (`KismetMathLibrary.MakeVector` 0.0 0.0 (- 0.0 (`self.DrownSpeed`))))))

(fn `Initialize`
  (params (TimeBeforeDrown :type "Float (double-precision)") (DrownSpeed :type "Float (double-precision)") (LifetimeAfterDrown :type "Float (double-precision)"))
  (set `self.TimeBeforeDrown` TimeBeforeDrown)
  (set `self.DrownSpeed` DrownSpeed)
  (set `self.LifetimeAfterDrown` LifetimeAfterDrown))

(fn `UserConstructionScript`)