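; Main menu game mode that sets up local multiplayer, with one controller and input receiver per PlayerStart.
; On BeginPlay it gathers all PlayerStarts, creates any missing local players, and possesses a BP_InputReceiver spawned at each start.
; The SpawnPlayer event spawns a sheep character at a given receiver's transform and hands that player controller over to it.
; Controller indices follow the order of the found starts; the TagToInt helper is not called here.
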(event `self.ReceiveBeginPlay`
  (`self.Get Player Starts`)
  (`self.SpawnInputReceivers`))

(event `/Game/Blueprints/GameMode/BPI_MainMenu.SpawnPlayer`
  (params (InputReceiver :type "/Game/Blueprints/Characters/BP_InputReceiver Object Reference") (PlayerController :type "PlayerController Object Reference"))
  (bind _returnvalue (`|SpawnActorFromClass` "/Game/Blueprints/Characters/BP_SheepCharacter.BP_SheepCharacter_C" (`self.GetTransform` InputReceiver) "Undefined" "MultiplyWithRoot" null null))
  (`Controller.Possess` PlayerController _returnvalue))

(fn `Get Player Starts`
  (bind _outactors (`GameplayStatics.GetAllActorsOfClass` "/Script/Engine.PlayerStart"))
  (set `self.PlayerStarts` _outactors))

(fn `SpawnInputReceivers`
  (locals (Index :type Integer))
  (for (_array_element _array_index) (`self.PlayerStarts`)
    (set `local.Index` _array_index)
    (if (not (`KismetSystemLibrary.IsValid` (`GameplayStatics.GetPlayerController` (`local.Index`))))
      (`GameplayStatics.CreatePlayer` (`local.Index`)))
    (bind _returnvalue (`|SpawnActorFromClass` "/Game/Blueprints/Characters/BP_InputReceiver.BP_InputReceiver_C" (`self.GetTransform` _array_element) "Undefined" "MultiplyWithRoot" null null))
    (`Controller.Possess` (`GameplayStatics.GetPlayerController` (`local.Index`)) _returnvalue)))

(fn `TagToInt`
  (params (Name :type "PlayerStart Object Reference"))
  (returns (Int :type Integer))
  (return (`KismetStringLibrary.Conv_StringToInt` (`KismetStringLibrary.Conv_NameToString` (`PlayerStart.PlayerStartTag` Name)))))

(fn `UserConstructionScript`)