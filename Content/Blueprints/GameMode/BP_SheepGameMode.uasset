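; Game mode for a local multiplayer sheep game that, on BeginPlay, sets up the players and a camera they all share.
; It randomly picks a player who has not yet been shepherd, rerolling against and updating the game instance's history.
; That player's controller possesses a new shepherd, the others possess sheep, and each views through the shared camera, which refreshes its targets.
; Finally, it has the game instance initialize the sheep count.
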(event `self.ReceiveBeginPlay`
  (`self.InitializeVariables`)
  (`self.SpawnCamera`)
  (`self.SpawnPlayers`)
  (`self.InitializeDataOnGameInstance`))

(fn `DefinePlayerCamera`
  (params (PlayerController :type "PlayerController Object Reference"))
  (`PlayerController.SetViewTargetWithBlend` PlayerController (`self.Camera`) 0.0 "VTBlend_Linear" 0.0 false)
  (`Camera.UpdateTargets` (`self.Camera`)))

(fn `GetRandomShepherdIndex`
  (returns (ShepherdIndex :type Integer))
  (locals (RandomIndex :type Integer :default 0))
  ;[0.2853 0.8177 0.5188 0.5] Get Random index while it already played as shepherd
  (bind _output_get (set `local.RandomIndex` (`KismetMathLibrary.RandomInteger` (`/Game/Blueprints/GameMode/BP_GameInstance.NbPlayers` (`self.GameInstance`))) :!label _label))
  (while (`|GetArrayItem` (`/Game/Blueprints/GameMode/BP_GameInstance.HavePlayedHasShepherd` (`self.GameInstance`)) (`local.RandomIndex`))
    (goto _label))
  (`KismetArrayLibrary.Array_Set` (`/Game/Blueprints/GameMode/BP_GameInstance.HavePlayedHasShepherd` (`self.GameInstance`)) _output_get true)
  (return _output_get))

(fn `InitializeDataOnGameInstance`
  (`/Game/Blueprints/GameMode/BP_GameInstance.InitializeNbSheeps` (`self.GameInstance`)))

(fn `InitializeVariables`
  (bind _asbp_game_instance (cast `/Game/Blueprints/GameMode/BP_GameInstance` (`GameplayStatics.GetGameInstance`)))
  (set `self.GameInstance` _asbp_game_instance))

(fn `SpawnCamera`
  (bind _returnvalue (`|SpawnActorFromClass` "/Game/Blueprints/Utils/Cameras/BP_SheepsCamera.BP_SheepsCamera_C" (`KismetMathLibrary.MakeTransform` (0.0 0.0 50.0)) "Undefined" "MultiplyWithRoot" null null))
  (set `self.Camera` _returnvalue))

(fn `SpawnPlayers`
  (locals (ShepherdIndex :type Integer :default 0))
  (bind _returnvalue (`KismetMathLibrary.MakeTransform` (0.0 0.0 0.0)))
  (set `local.ShepherdIndex` (`self.GetRandomShepherdIndex`))
  (for _index (range (`/Game/Blueprints/GameMode/BP_GameInstance.NbPlayers` (`self.GameInstance`)))
    (if (== (`local.ShepherdIndex`) _index)
      (bind _returnvalue_2 (`|SpawnActorFromClass` "/Game/Blueprints/Characters/BP_ShepherdCharacter.BP_ShepherdCharacter_C" _returnvalue "Undefined" "MultiplyWithRoot" null null))
      (bind _returnvalue_3 (`GameplayStatics.GetPlayerController` _index))
      (`Controller.Possess` _returnvalue_3 _returnvalue_2)
      (else
        (bind _returnvalue_4 (`|SpawnActorFromClass` "/Game/Blueprints/Characters/BP_SheepCharacter.BP_SheepCharacter_C" _returnvalue "Undefined" "MultiplyWithRoot" null null))
        (`Controller.Possess` _returnvalue_3 _returnvalue_4)))
    (`self.DefinePlayerCamera` _returnvalue_3)))

(fn `UserConstructionScript`)