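; Main menu game mode that sets up local multiplayer with sheep characters and a shared sheep camera.
; On BeginPlay it creates any missing local players up to the GameInstance maximum and spawns an input receiver for each.
; Already-present players possess sheep spawned at transforms from TakeSheepBotPlace, while other slots possess their receivers.
; The SpawnPlayer event later gives a controller a sheep and updates the camera targets.
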(event `self.ReceiveBeginPlay`
  (`self.InitializeVariables`)
  (`self.SpawnCamera`)
  (`self.SpawnPlayers`))

(event `/Game/Blueprints/GameMode/MainMenu/BPI_MainMenu.SpawnPlayer`
  (params (InputReceiver :type "/Game/Blueprints/Characters/BP_InputReceiver Object Reference") (PlayerController :type "PlayerController Object Reference"))
  (`self.SpawnSheepCharacter` PlayerController))

(fn `InitializeVariables`
  (bind _asbp_game_instance (cast `/Game/Blueprints/GameMode/BP_GameInstance` (`GameplayStatics.GetGameInstance`)))
  (set `self.GameInstance` _asbp_game_instance))

(fn `SetPlayerControllerCamera`
  (params (`Player Controller` :type "PlayerController Object Reference"))
  (`PlayerController.SetViewTargetWithBlend` `Player Controller` (`self.Camera`) 0.0 "VTBlend_Linear" 0.0 false)
  (`Camera.UpdateTargets` (`self.Camera`)))

(fn `SpawnCamera`
  (bind _returnvalue (`|SpawnActorFromClass` "/Game/Blueprints/Utils/Cameras/BP_SheepsCamera.BP_SheepsCamera_C" (`KismetMathLibrary.MakeTransform` (0.0 0.0 50.0)) "Undefined" "MultiplyWithRoot" null null))
  (set `self.Camera` _returnvalue))

(fn `SpawnInputReceivers`
  (params (IsPlayerControllerValid :type Boolean) (Index :type Integer))
  (returns (InputReceiver :type "/Game/Blueprints/Characters/BP_InputReceiver Object Reference"))
  (if (not IsPlayerControllerValid)
    (`GameplayStatics.CreatePlayer` Index))
  (bind _returnvalue (`|SpawnActorFromClass` "/Game/Blueprints/Characters/BP_InputReceiver.BP_InputReceiver_C" (`KismetMathLibrary.MakeTransform` (0.0 0.0 0.0)) "Undefined" "MultiplyWithRoot" null null))
  (return _returnvalue))

(fn `SpawnPlayers`
  (locals (Index :type Integer) (InputReceiver :type "/Game/Blueprints/Characters/BP_InputReceiver Object Reference"))
  (bind _returnvalue (`GameplayStatics.GetPlayerController` (`local.Index`)))
  (for _index (range (`/Game/Blueprints/GameMode/BP_GameInstance.NbPlayersMax` (`self.GameInstance`)))
    (bind _output_get (set `local.Index` _index))
    (bind _inputreceiver (`self.SpawnInputReceivers` (`KismetSystemLibrary.IsValid` (`GameplayStatics.GetPlayerController` (`local.Index`))) _output_get))
    ;[0.2853 0.8177 0.5188 0.5] If player already present : Control a Sheep             Else : Control an input Receiver
    (set `local.InputReceiver` _inputreceiver)
    (if (> (`/Game/Blueprints/GameMode/BP_GameInstance.NbPlayers` (`self.GameInstance`)) (`local.Index`))
      (`self.SpawnSheepCharacter` (`GameplayStatics.GetPlayerController` (`local.Index`)))
      (else
        (`Controller.Possess` _returnvalue (`local.InputReceiver`))
        (`self.SetPlayerControllerCamera` _returnvalue)))))

(fn `SpawnSheepCharacter`
  (params (PlayerController :type "PlayerController Object Reference"))
  (bind _sheeptransform (`/Game/Blueprints/GameMode/BP_GameInstance.TakeSheepBotPlace` (`self.GameInstance`)))
  (bind _returnvalue (`|SpawnActorFromClass` "/Game/Blueprints/Characters/BP_SheepCharacter.BP_SheepCharacter_C" _sheeptransform "Undefined" "MultiplyWithRoot" null null))
  (`Controller.Possess` PlayerController _returnvalue)
  (`self.SetPlayerControllerCamera` PlayerController))

(fn `TagToInt`
  (params (Name :type "PlayerStart Object Reference"))
  (returns (Int :type Integer))
  (return (`KismetStringLibrary.Conv_StringToInt` (`KismetStringLibrary.Conv_NameToString` (`PlayerStart.PlayerStartTag` Name)))))

(fn `UserConstructionScript`)