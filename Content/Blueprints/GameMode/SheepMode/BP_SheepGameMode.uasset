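; Game mode for the local multiplayer Sheep mode, where one player is the shepherd and the others are sheep.
; On BeginPlay it spawns a shared camera, spawns and possesses player characters, then initializes sheep through the GameInstance.
; The shepherd is picked by random retry among players yet to play that role, tracked in the GameInstance.
; The shepherd spawns at a PlayerStart, while player sheep take sheep bot places.
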(event `self.ReceiveBeginPlay`
  (`self.InitializeVariables`)
  (`self.SpawnCamera`)
  (`self.SpawnPlayers`)
  (`MainGameInstance.InitializeSheeps` (`self.GameInstance`)))

(fn `DefinePlayerCamera`
  (params (PlayerController :type "PlayerController Object Reference"))
  (`PlayerController.SetViewTargetWithBlend` PlayerController (`self.Camera`) 0.0 "VTBlend_Linear" 0.0 false)
  (`Camera.UpdateTargets` (`self.Camera`)))

(fn `GetRandomShepherdIndex`
  (returns (ShepherdIndex :type Integer))
  (locals (RandomIndex :type Integer :default 0))
  ;[0.2853 0.8177 0.5188 0.5] Get Random index while it already played as shepherd
  (set `local.RandomIndex` (`.OutIndex` (`KismetArrayLibrary.Array_Random` (`/Game/Blueprints/GameMode/BP_GameInstance.PlayersId` (`self.GameInstance`)))) :!label _label)
  (while (`|GetArrayItem` (`/Game/Blueprints/GameMode/BP_GameInstance.HavePlayedHasShepherd` (`self.GameInstance`)) (`local.RandomIndex`))
    (goto _label))
  ;[0.2853 0.8177 0.5188 0.5] Set have played has shepherd value to true
  (`KismetArrayLibrary.Array_Set` (`/Game/Blueprints/GameMode/BP_GameInstance.HavePlayedHasShepherd` (`self.GameInstance`)) (`local.RandomIndex`) true)
  (return (`|GetArrayItem` (`/Game/Blueprints/GameMode/BP_GameInstance.PlayersId` (`self.GameInstance`)) (`local.RandomIndex`))))

(fn `InitializeVariables`
  (bind _asbp_game_instance (cast `/Game/Blueprints/GameMode/BP_GameInstance` (`GameplayStatics.GetGameInstance`)))
  (set `self.GameInstance` _asbp_game_instance))

(fn `PossessPawn`
  (params (InPawn :type "Pawn Object Reference") (PlayerController :type "PlayerController Object Reference"))
  (`Controller.Possess` PlayerController InPawn)
  (`self.DefinePlayerCamera` PlayerController))

(fn `SpawnCamera`
  (bind _returnvalue (`|SpawnActorFromClass` "/Game/Blueprints/Gameplay/Cameras/BP_SheepsCamera.BP_SheepsCamera_C" (`KismetMathLibrary.MakeTransform` (0.0 0.0 50.0)) "Undefined" "MultiplyWithRoot" null null))
  (set `self.Camera` _returnvalue)
  ;[0.3133 0.7537 0.8281 0.5] Set camera as possessed for all player controller event if there are not used
  (for _index (range 4)
    (bind _returnvalue_2 (`GameplayStatics.GetPlayerController` _index))
    (`/Engine/EditorBlueprintResources/StandardMacros.IsValid` _returnvalue_2
      (:`Is Valid`
        (`self.DefinePlayerCamera` _returnvalue_2)))))

(fn `SpawnPlayers`
  (locals (ShepherdIndex :type Integer :default 0))
  (set `local.ShepherdIndex` (`self.GetRandomShepherdIndex`))
  (for _array_element (`/Game/Blueprints/GameMode/BP_GameInstance.PlayersId` (`self.GameInstance`))
    (if (== _array_element (`local.ShepherdIndex`))
      (bind _returnvalue (`GameplayStatics.GetPlayerController` _array_element))
      (`self.SpawnShepherdCharacter` _returnvalue)
      (else
        (`self.SpawnSheepCharacter` _returnvalue)))))

(fn `SpawnSheepCharacter`
  (params (PlayerController :type "PlayerController Object Reference"))
  (bind _sheeptransform (`/Game/Blueprints/GameMode/BP_GameInstance.TakeSheepBotPlace` (`self.GameInstance`)))
  (bind _returnvalue (`|SpawnActorFromClass` "/Game/Blueprints/Characters/BP_SheepCharacter.BP_SheepCharacter_C" _sheeptransform "Undefined" "MultiplyWithRoot" null null))
  (`self.PossessPawn` _returnvalue (`local.PlayerController`)))

(fn `SpawnShepherdCharacter`
  (params (PlayerController :type "PlayerController Object Reference"))
  (bind _returnvalue (`GameplayStatics.GetActorOfClass` "/Script/Engine.PlayerStart"))
  (bind _returnvalue_2 (`|SpawnActorFromClass` "/Game/Blueprints/Characters/BP_ShepherdCharacter.BP_ShepherdCharacter_C" (`self.GetTransform` _returnvalue) "Undefined" "MultiplyWithRoot" null null))
  (`self.PossessPawn` _returnvalue_2 (`local.PlayerController`))
  (set `MainGameInstance.Shepherd` _returnvalue_2 (`self.GameInstance`)))

(fn `UserConstructionScript`)