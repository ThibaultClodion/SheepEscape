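; Game mode for a test map that cycles through numbered shepherd-and-sheep scenarios, with a UI widget showing the current test.
; On BeginPlay it spawns a shared camera and a shepherd possessed by the first player.
; Each test respawns sheep bots, teleports the shepherd, and gives other players sheep characters in bot places.
; Layouts are TargetPoints and PlayerStarts matched by their display name's first character; Next/Previous wrap on PlayerStart count.
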(event `self.ReceiveBeginPlay`
  (`self.InitializeVariables`)
  (`self.SpawnUI`)
  (`self.SpawnCamera`)
  (`self.SpawnShepherd`)
  (`self.SpawnTest`))

(fn `DestroyOldSheeps`
  (bind _outactors (`GameplayStatics.GetAllActorsOfClass` "/Game/Blueprints/Characters/BP_SheepBot.BP_SheepBot_C"))
  (for _array_element _outactors
    (`self.K2_DestroyActor` _array_element)))

(fn `InitializeVariables`
  (bind _asbp_game_instance (cast `/Game/Blueprints/GameMode/BP_GameInstance` (`GameplayStatics.GetGameInstance`)))
  (set `self.GameInstance` _asbp_game_instance))

(fn `NextTest`
  (bind _outactors (`GameplayStatics.GetAllActorsOfClass` "/Script/Engine.PlayerStart"))
  (set `self.ActualTest` (mod (+ (`self.ActualTest`) 1) (`KismetArrayLibrary.Array_Length` _outactors)))
  (`self.SpawnTest`))

(fn `PreviousTest`
  (bind _outactors (`GameplayStatics.GetAllActorsOfClass` "/Script/Engine.PlayerStart"))
  (bind _returnvalue (`KismetArrayLibrary.Array_Length` _outactors))
  (set `self.ActualTest` (mod (+ (mod (- (`self.ActualTest`) 1) _returnvalue) _returnvalue) _returnvalue))
  (`self.SpawnTest`))

(fn `SpawnCamera`
  (bind _returnvalue (`|SpawnActorFromClass` "/Game/Blueprints/Gameplay/Cameras/BP_SheepsCamera.BP_SheepsCamera_C" (`KismetMathLibrary.MakeTransform` (0.0 0.0 50.0)) "Undefined" "MultiplyWithRoot" null null))
  (set `self.Camera` _returnvalue)
  ;[0.3133 0.7537 0.8281 0.5] Set camera as possessed for all player controller event if there are not used
  (for _index (range 4)
    (bind _returnvalue_2 (`GameplayStatics.GetPlayerController` _index))
    (`/Engine/EditorBlueprintResources/StandardMacros.IsValid` _returnvalue_2
      (:`Is Valid`
        (`PlayerController.SetViewTargetWithBlend` _returnvalue_2 (`self.Camera`) 0.0 "VTBlend_Linear" 0.0 false)
        (`Camera.UpdateTargets` (`self.Camera`))))))

(fn `SpawnSheeps`
  (bind _outactors (`GameplayStatics.GetAllActorsOfClass` "/Script/Engine.TargetPoint"))
  (for _array_element _outactors
    (if (== (`KismetStringLibrary.GetSubstring` (`KismetSystemLibrary.GetDisplayName` _array_element)) (`KismetStringLibrary.Conv_IntToString` (`self.ActualTest`)))
      (`|SpawnActorFromClass` "/Game/Blueprints/Characters/BP_SheepBot.BP_SheepBot_C" (`self.GetTransform` _array_element) "Undefined" "MultiplyWithRoot" null null))))

(fn `SpawnShepherd`
  (bind _returnvalue (`GameplayStatics.GetPlayerController` (`|GetArrayItem` (`/Game/Blueprints/GameMode/BP_GameInstance.PlayersId` (`self.GameInstance`)))))
  (bind _outactors (`GameplayStatics.GetAllActorsOfClass` "/Script/Engine.PlayerStart"))
  (for _array_element _outactors
    (if (== (`KismetStringLibrary.GetSubstring` (`KismetSystemLibrary.GetDisplayName` _array_element)) "0")
      (bind _returnvalue_2 (`|SpawnActorFromClass` "/Game/Blueprints/Characters/BP_ShepherdCharacter.BP_ShepherdCharacter_C" (`self.GetTransform` _array_element) "Undefined" "MultiplyWithRoot" null null))
      (`Controller.Possess` _returnvalue _returnvalue_2)
      (`PlayerController.SetViewTargetWithBlend` _returnvalue (`self.Camera`) 0.0 "VTBlend_Linear" 0.0 false)
      (`Camera.UpdateTargets` (`self.Camera`)))))

(fn `SpawnTest`
  (`self.DestroyOldSheeps`)
  (`self.SpawnSheeps`)
  (`self.TeleportShepherd`)
  (`self.TakeSheepBotPlace`)
  (`self.UpdateGameInstance`)
  (`self.UpdateTestText`)
  (`Camera.UpdateTargets` (`self.Camera`)))

(fn `SpawnUI`
  (bind _returnvalue (`|CreateWidget` "/Game/Blueprints/GameMode/Test/WB_Testmap.WB_Testmap_C"))
  (bind _output_get (set `self.Widget` _returnvalue))
  (`UserWidget.AddToViewport` _output_get 0)
  (set `PlayerController.bShowMouseCursor` true (`GameplayStatics.GetPlayerController` 0)))

(fn `TakeSheepBotPlace`
  (for (_array_element _array_index) (`/Game/Blueprints/GameMode/BP_GameInstance.PlayersId` (`self.GameInstance`))
    ;[0.3986 0.8229 0.5834 0.5] First Element is Shepherd (on test)
    (if (> _array_index 0)
      (bind _sheeptransform (`/Game/Blueprints/GameMode/BP_GameInstance.TakeSheepBotPlace` (`self.GameInstance`)))
      (bind _returnvalue (`|SpawnActorFromClass` "/Game/Blueprints/Characters/BP_SheepCharacter.BP_SheepCharacter_C" _sheeptransform "Undefined" "MultiplyWithRoot" null null))
      (bind _returnvalue_2 (`GameplayStatics.GetPlayerController` _array_element))
      (`Controller.Possess` _returnvalue_2 _returnvalue)
      (`PlayerController.SetViewTargetWithBlend` _returnvalue_2 (`self.Camera`) 0.0 "VTBlend_Linear" 0.0 false)
      (`Camera.UpdateTargets` (`self.Camera`)))))

(fn `TeleportShepherd`
  (bind _outactors (`GameplayStatics.GetAllActorsOfClass` "/Script/Engine.PlayerStart"))
  (for _array_element _outactors
    (if (== (`KismetStringLibrary.GetSubstring` (`KismetSystemLibrary.GetDisplayName` _array_element)) (`KismetStringLibrary.Conv_IntToString` (`self.ActualTest`)))
      (bind _returnvalue (`GameplayStatics.GetActorOfClass` "/Game/Blueprints/Characters/BP_ShepherdCharacter.BP_ShepherdCharacter_C"))
      (`self.K2_SetActorTransform` _returnvalue (`self.GetTransform` _array_element) false true))))

(fn `UpdateGameInstance`
  (bind _gameinstance (`self.GameInstance`))
  (`MainGameInstance.InitializeSheeps` _gameinstance)
  (bind _returnvalue (`GameplayStatics.GetActorOfClass` "/Game/Blueprints/Characters/BP_ShepherdCharacter.BP_ShepherdCharacter_C"))
  (set `MainGameInstance.Shepherd` _returnvalue _gameinstance))

(fn `UpdateTestText`
  (`/Game/Blueprints/GameMode/Test/WB_Testmap.ChangeText` (`self.Widget`) (`self.ActualTest`)))

(fn `UserConstructionScript`)