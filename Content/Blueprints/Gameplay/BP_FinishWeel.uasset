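; Finish zone that ends the round once every sheep is inside its sphere trigger.
; Overlap events keep a count of sheep bots and sheep characters, seeded shortly after BeginPlay to catch those already overlapping.
; Each begin overlap compares that count to the GameInstance sheep total.
; On a match, it adds one rescue score per sheep to the shepherd, then calls EndRound on the GameInstance.
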(event `self.ReceiveBeginPlay`
  (`self.InitializeVariables`)
  ;[0.2853 0.8177 0.5188 0.5] Necessary to let time for checking already overlapping sheeps
  (`KismetSystemLibrary.Delay` 0.2)
  (`self.GetAlreadyOverlappingSheeps`))

(event `self.Sphere.OnComponentBeginOverlap`
  (params (OverlappedComponent :type "PrimitiveComponent Object Reference") (OtherActor :type "Actor Object Reference") (OtherComp :type "PrimitiveComponent Object Reference") (OtherBodyIndex :type Integer) (bFromSweep :type Boolean) (SweepResult :type "HitResult Structure (by ref)"))
  (`self.ActorOverlap` OtherActor)
  (`self.CheckIfAllSheepsRescue`))

(event `self.Sphere.OnComponentEndOverlap`
  (params (OverlappedComponent :type "PrimitiveComponent Object Reference") (OtherActor :type "Actor Object Reference") (OtherComp :type "PrimitiveComponent Object Reference") (OtherBodyIndex :type Integer))
  (`self.ActorEndOverlap` OtherActor))

(fn `ActorEndOverlap`
  (params (Actor :type "Object Object Reference"))
  (cast `/Game/Blueprints/Characters/BP_SheepBot` Actor
    (:`then`
      _)
    (:`CastFailed`
      (cast `/Game/Blueprints/Characters/BP_SheepCharacter` Actor)))
  (`/Engine/EditorBlueprintResources/StandardMacros.DecrementInt` (`self.NbSheepsInside`)))

(fn `ActorOverlap`
  (params (Actor :type "Object Object Reference"))
  (cast `/Game/Blueprints/Characters/BP_SheepBot` Actor
    (:`then`
      _)
    (:`CastFailed`
      (cast `/Game/Blueprints/Characters/BP_SheepCharacter` Actor)))
  (`/Engine/EditorBlueprintResources/StandardMacros.IncrementInt` (`self.NbSheepsInside`)))

(fn `AddSheepRescuesScore`
  (locals (Shepherd :type "/Game/Blueprints/Characters/BP_ShepherdCharacter Object Reference"))
  (bind _returnvalue (`GameplayStatics.GetActorOfClass` "/Game/Blueprints/Characters/BP_ShepherdCharacter.BP_ShepherdCharacter_C"))
  (set `local.Shepherd` _returnvalue)
  (for _ (range (`self.NbSheepsInside`))
    (`/Game/Blueprints/Characters/BP_ShepherdCharacter.AddSheepRescueScore` (`local.Shepherd`))))

(fn `CheckIfAllSheepsRescue`
  (if (== (`self.NbSheepsInside`) (`/Game/Blueprints/GameMode/BP_GameInstance.NbSheeps` (`self.GameInstance`)))
    (`self.AddSheepRescuesScore`)
    (`/Game/Blueprints/GameMode/BP_GameInstance.EndRound` (`self.GameInstance`) true)))

(fn `GetAlreadyOverlappingSheeps`
  (set `self.NbSheepsInside` (+ (`KismetArrayLibrary.Array_Length` (`PrimitiveComponent.GetOverlappingActors` (`self.Sphere`) "/Game/Blueprints/Characters/BP_SheepBot.BP_SheepBot_C")) (`KismetArrayLibrary.Array_Length` (`PrimitiveComponent.GetOverlappingActors` (`self.Sphere`) "/Game/Blueprints/Characters/BP_SheepCharacter.BP_SheepCharacter_C")))))

(fn `InitializeVariables`
  (bind _asbp_game_instance (cast `/Game/Blueprints/GameMode/BP_GameInstance` (`GameplayStatics.GetGameInstance`)))
  (set `self.GameInstance` _asbp_game_instance))

(fn `UserConstructionScript`)