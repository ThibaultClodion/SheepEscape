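; BP_BaseSign is a base sign Blueprint that runs an action once all players are in.
; AllPlayerin starts a three-second retriggerable delay, then rechecks the player-in count against the GameInstance's player total before calling ExecuteFunction, which is empty here.
; CancelAllPlayerin retriggers the same delay at zero, so the guard on the delay value skips execution.
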(event `self.ReceiveBeginPlay`
  (`self.InitializeVariables`))

(event `self.AllPlayerIn`
  (set `self.PlayDelay` 3.0)
  ; TODO : Add a Countdown Widget
  (`KismetSystemLibrary.RetriggerableDelay` (`self.PlayDelay`) :!label _label)
  (if (> (`self.PlayDelay`) 0.01)
    ; Check if all player really in
    (bind _bool (`self.AreAllPlayersIn`))
    (if _bool
      (`self.ExecuteFunction`))))

(event `self.CancelAllPlayerIn`
  (set `self.PlayDelay` 0.0)
  (goto _label))

(fn `AreAllPlayersIn`
  (returns (Bool :type Boolean))
  (return (== (`/Game/Blueprints/GameMode/BP_GameInstance.NbPlayers` (`self.GameInstance`)) (`self.PlayerIn`))))

(fn `ExecuteFunction`)

(fn `InitializeVariables`
  (bind _asbp_game_instance (cast `/Game/Blueprints/GameMode/BP_GameInstance` (`GameplayStatics.GetGameInstance`)))
  (set `self.GameInstance` _asbp_game_instance))

(fn `UserConstructionScript`)