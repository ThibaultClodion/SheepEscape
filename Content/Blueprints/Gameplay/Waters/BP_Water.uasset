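; BP_Water is a water hazard that eliminates characters entering its EliminationBox.
; Any overlapping actor triggers a splash effect and sound and spawns a BP_SheepInWater at its transform, before the BaseCharacter cast and Eliminate call.
; The spawned sheep receives a direction derived from the negated cosine and sine of the water plane's yaw, plus speed and drowning settings, then drops into the water.
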(event `self.EliminationBox.OnComponentBeginOverlap`
  (params (OverlappedComponent :type "PrimitiveComponent Object Reference") (OtherActor :type "Actor Object Reference") (OtherComp :type "PrimitiveComponent Object Reference") (OtherBodyIndex :type Integer) (bFromSweep :type Boolean) (SweepResult :type "HitResult Structure (by ref)"))
  (`self.SpawnSheepInWater` OtherActor)
  (bind _asbase_character (cast `BaseCharacter` OtherActor))
  (`BaseCharacter.Eliminate` _asbase_character))

(fn `PlayEffects`
  (params (Transform :type "Transform Structure"))
  (bind _transform_location (`KismetMathLibrary.BreakTransform` (`local.Transform`)))
  (`NiagaraFunctionLibrary.SpawnSystemAtLocation` "/Game/Assets/FX/Water/NS_Water_Drop.NS_Water_Drop" Transform_Location Transform_Rotation Transform_Scale)
  (`GameplayStatics.PlaySoundAtLocation` "/Game/Assets/MetaSounds/SFX/Nature/MS_Splash.MS_Splash" _transform_location (struct) 1.0 1.0 0.0 null null null null))

(fn `RotationToDirection`
  (returns (Direction :type "Vector Structure"))
  (bind (_returnvalue_roll _returnvalue_pitch _returnvalue_yaw) (`KismetMathLibrary.BreakRotator` (`SceneComponent.K2_GetComponentRotation` (`self.SM_Water_Plane`))))
  (return (`KismetMathLibrary.MakeVector` (- 0.0 (`KismetMathLibrary.Cos` _returnvalue_yaw)) (- 0.0 (`KismetMathLibrary.Sin` _returnvalue_yaw)))))

(fn `SpawnSheepInWater`
  (params (EliminateActor :type "Actor Object Reference"))
  (bind _returnvalue (`self.GetTransform` EliminateActor))
  (`self.PlayEffects` _returnvalue)
  (bind _returnvalue_2 (`|SpawnActorFromClass` "/Game/Blueprints/Characters/BP_SheepInWater.BP_SheepInWater_C" _returnvalue "Undefined" "MultiplyWithRoot" null null))
  (`/Game/Blueprints/Characters/BP_SheepInWater.Initialize` _returnvalue_2 (`self.RotationToDirection`) (`self.SheepSpeed`) (`self.SheepTimeBeforeDrown`) (`self.SheepDrownSpeed`) (`self.SheepLifeTimeAfterDrown`))
  (`/Game/Blueprints/Characters/BP_SheepInWater.DropInWater` _returnvalue_2))

(fn `UserConstructionScript`)