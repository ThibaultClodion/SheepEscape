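; BP_FinishWeel is the finish variant of a "Weel" actor that ends the round once all sheep are in.
; It caches the BP_GameInstance on BeginPlay.
; On the AllSheepsin event, it calls AddSheepRescueScore on the BP_ShepherdCharacter once per sheep counted in NbSheepsInside, then calls EndRound with true on the game instance.
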(event `self.ReceiveBeginPlay`
  (`self.InitializeVariables`))

(event `self.AllSheepsIn`
  (`self.AddSheepRescueScores`)
  (`/Game/Blueprints/GameMode/BP_GameInstance.EndRound` (`self.GameInstance`) true))

(fn `AddSheepRescueScores`
  (locals (Shepherd :type "/Game/Blueprints/Characters/BP_ShepherdCharacter Object Reference"))
  (bind _returnvalue (`GameplayStatics.GetActorOfClass` "/Game/Blueprints/Characters/BP_ShepherdCharacter.BP_ShepherdCharacter_C"))
  (set `local.Shepherd` _returnvalue)
  (for _ (range (`self.NbSheepsInside`))
    (`/Game/Blueprints/Characters/BP_ShepherdCharacter.AddSheepRescueScore` (`local.Shepherd`))))

(fn `InitializeVariables`
  (bind _asbp_game_instance (cast `/Game/Blueprints/GameMode/BP_GameInstance` (`GameplayStatics.GetGameInstance`)))
  (set `self.GameInstance` _asbp_game_instance))

(fn `UserConstructionScript`)